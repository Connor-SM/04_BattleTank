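; Player-controllable tank Blueprint that routes input to its track, movement, camera and firing functions.
; On BeginPlay it passes its Barrel and Turret components to the reference setters used by the tank.
; Throttle axes drive each track separately, while a forward/backward axis feeds TankMovementComponent's IntendMoveForward.
; Aim axes rotate the azimuth gimbal in yaw and spring arm in pitch, scaled by delta time, and the Fire action calls Fire.
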(event EventBeginPlay
  (Class|Tank|SetBarrelReference (Variables|Default|GetBarrel))
  (Class|Tank|SetTurretReference (Variables|Default|GetTurret)))

(event Collision|EventActorBeginOverlap
  (params (OtherActor :type Actor%20Object%20Reference)))

(event EventTick
  (params (DeltaSeconds :type Float%20%28single-precision%29)))

(event Input|ActionEvents|InputActionFire
  (params (Key :type Key%20Structure :default "AnyKey"))
  ;[1 1 1] Aim Input Binding
  ;;[1 1 1] To Fire the Missile - Input
  (:Pressed
    (Class|Tank|Fire)))

(event Input|AxisEvents|InputAxisAimElevation
  (params (AxisValue :type Float%20%28single-precision%29))
  ;[1 1 1] Aim Input Binding
  ;;[1 1 1] For Camera Rotation on 'Y' Axis
  (Transformation|AddLocalRotation (Variables|Default|GetSpringArm) (Math|Rotator|MakeRotator 0.0 (* AxisValue (Utilities|Time|GetWorldDeltaSeconds) 1e+02) 0.0) false false))

(event Input|AxisEvents|InputAxisForward&BackwardMovement
  (params (AxisValue :type Float%20%28single-precision%29))
  ;[1 1 1] Input for Tracks for Mobility
  (Class|TankMovementComponent|IntendMoveForward (Variables|Default|GetTankMovementComponent) AxisValue))

(event Input|AxisEvents|InputAxisLeftTrackThrottle
  (params (AxisValue :type Float%20%28single-precision%29))
  ;[1 1 1] Input for Tracks for Mobility
  (Class|TankTrack|SetThrottle (Variables|Default|GetLeft%20Track) AxisValue))

(event Input|AxisEvents|InputAxisRightTrackThrottle
  (params (AxisValue :type Float%20%28single-precision%29))
  ;[1 1 1] Input for Tracks for Mobility
  (Class|TankTrack|SetThrottle (Variables|Default|GetRight%20Track) AxisValue))

(event Input|AxisEvents|InputAxisAimAzimuth
  (params (AxisValue :type Float%20%28single-precision%29))
  ;[1 1 1] Aim Input Binding
  ;;[1 1 1] For Camera Rotation on 'X' Axis
  (Transformation|AddLocalRotation (Variables|Default|GetAzimuth%20Gimbal) (Math|Rotator|MakeRotator 0.0 0.0 (* AxisValue (Utilities|Time|GetWorldDeltaSeconds) 1e+02)) false false))

(fn ConstructionScript)